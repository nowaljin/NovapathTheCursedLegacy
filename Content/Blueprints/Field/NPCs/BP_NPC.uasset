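; BP_NPC is a field NPC the player can always interact with to start a conversation.
; On BeginPlay it applies its Skin to the base layer of its animation instance.
; Interacting passes itself and its DialogueRow to the game mode through a conversation interface message, and it supplies CharName as the speaker name.
; Its ID getter returns a fixed "None".
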(event `self.ReceiveBeginPlay`
  (`PaperZDAnimInstance.ApplyAnimationSkinToLayer` (`PaperZDAnimationComponent.AnimInstance` (`self.AnimationComponent`)) (`self.Skin`) 0))

(event `/Game/Definitions/Interfaces/BPI_Interactable.I_Interact`
  (message `/Game/Definitions/Interfaces/BPI_DialogueControl.I_StartConversation` (`GameplayStatics.GetGameMode`) self (`self.DialogueRow`)))

(fn `I_CanInteract`
  (returns (CanInteract :type Boolean))
  (return true))

(fn `I_GetID`
  (returns (ID :type Name))
  (return "None"))

(fn `I_GetSpeakerName`
  (returns (SpeakerName :type Text))
  (return (`self.CharName`)))

(fn `UserConstructionScript`)