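; Base Blueprint for a party member character in the field, drawn as a sprite with a swappable animation Blueprint.
; BeginPlay creates a dynamic material instance on the sprite.
; ApplyMemberData stores the member's data and ID, sets that member's field anim class, and feeds the ID into the material's DepthOffset parameter, giving each member its own depth offset.
; A helper returns the length of the velocity vector.
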(event `self.ReceiveBeginPlay`
  (bind _returnvalue (`PrimitiveComponent.CreateDynamicMaterialInstance` (`self.Sprite`) 0 null "None"))
  (set `self.DynamicSpriteMat` _returnvalue))

(fn `ApplyMemberData`
  (params (MemberData :type "/Game/Data/DataAssets/PartyMemberData/PDA_PartyMemberData Object Reference") (MemberID :type Integer))
  (set `self.MemberData` MemberData)
  (`PaperZDAnimationComponent.SetAnimInstanceClass` (`self.AnimationComponent`) (`/Game/Data/DataAssets/PartyMemberData/PDA_PartyMemberData.FieldAnimBP` (`self.MemberData`)))
  (set `self.Member ID` (`local.MemberID`))
  (`MaterialInstanceDynamic.SetScalarParameterValue` (`self.DynamicSpriteMat`) "DepthOffset" (`KismetMathLibrary.Conv_IntToDouble` (`local.MemberID`))))

(fn `GetCustomVelocityLenght`
  (returns (ReturnValue :type "Float (double-precision)"))
  (return (`KismetMathLibrary.VSize` (`self.GetVelocity`))))

(fn `UserConstructionScript`)