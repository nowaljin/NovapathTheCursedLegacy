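; BP_FieldFollower is a field actor that trails a FollowTarget by replaying that target's recorded movement.
; Each tick it requests the entry for its MemberID from the target's ACMoveHistory and, if valid, interpolates its transform toward it without sweep.
; Because it moves by setting transforms, it derives its own floored speed from position change over delta time, exposed through GetCustomVelocityLenght.
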(event `self.ReceiveBeginPlay`
  (`parent.ReceiveBeginPlay`)
  (set `self.LastLocation` (`self.K2_GetActorLocation`)))

(event `self.ReceiveTick`
  (params (DeltaSeconds :type "Float (single-precision)"))
  (`parent.ReceiveTick` DeltaSeconds)
  (bind _followtarget (`self.FollowTarget`)
    (:`then`
      (bind (_targettransform _isvalid) (`/Game/Blueprints/Components/AC_MoveHistory.GetEntryForMemberIndex` (`/Game/Blueprints/Field/BP_FieldPlayer.AC_MoveHistory` _followtarget) (`self.Member ID`)))
      (if _isvalid
        (set `self.Target Transform` _targettransform)
        (`self.UpdateVelocity`)
        (`self.K2_SetActorTransform` (`KismetMathLibrary.TInterpTo` (`self.GetTransform`) (`self.Target Transform`) (`GameplayStatics.GetWorldDeltaSeconds`) (`self.MoveInterpSpeed`)))))
    (:`else`)))

(fn `GetCustomVelocityLenght`
  (returns (ReturnValue :type "Float (double-precision)"))
  (return (`self.CustomVelocityLenght`)))

(fn `UpdateVelocity`
  (set `self.CustomVelocityLenght` (`KismetMathLibrary.Conv_IntToDouble` (`KismetMathLibrary.FFloor` (/ (`KismetMathLibrary.Vector_Distance` (`self.K2_GetActorLocation`) (`self.LastLocation`)) (`GameplayStatics.GetWorldDeltaSeconds`)))))
  (set `self.LastLocation` (`self.K2_GetActorLocation`)))

(fn `UserConstructionScript`
  (`parent.UserConstructionScript`))