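; AC_MoveHistory is a component that keeps a rolling history of transforms, indexed by member ID, apparently for followers trailing a path.
; AddTransform appends to PastTransforms and drops the oldest entry once MaxEntries is exceeded.
; GetEntryForMemberIndex steps back from the newest entry by MemberID times EntrySteps, returning that transform or an invalid flag if history is too short.
; It does not tick; recording depends on external calls.
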(fn `AddTransform`
  (params (TransformToAdd :type "Transform Structure"))
  (`KismetArrayLibrary.Array_Add` (`self.PastTransforms`) TransformToAdd)
  (if (> (`KismetArrayLibrary.Array_Length` (`self.PastTransforms`)) (`self.MaxEntries`))
    (`KismetArrayLibrary.Array_Remove` (`self.PastTransforms`))))

(fn `GetEntryForMemberIndex`
  (params (MemberID :type Integer))
  (returns (TargetTransform :type "Transform Structure (by ref)") (IsValid :type Boolean))
  (locals (CheckEnrty :type Integer))
  (set `local.CheckEnrty` (- (`KismetArrayLibrary.Array_LastIndex` (`self.PastTransforms`)) (* MemberID (`self.EntrySteps`))))
  (if (`KismetArrayLibrary.Array_IsValidIndex` (`self.PastTransforms`) (`local.CheckEnrty`))
    (return (`|GetArrayItem` (`self.PastTransforms`) (`local.CheckEnrty`)) true)
    (else
      (return (struct) false))))