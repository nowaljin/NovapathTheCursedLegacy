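; Dialogue manager component that runs linear conversations between the player and a target actor from rows in DT_Dialogue.
; StartConversation shows the first line and conversation-locks both participants through interface messages.
; ProgressConversation follows each row's NextRow, ending and unlocking on "None" or a missing row.
; Lines display through a widget obtained from the PlayerController, with IsPlayer choosing the speaker.
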(fn `EndConversation`
  (message `/Game/Definitions/Interfaces/BPI_DialogueControl.I_SetConversationLock` (`GameplayStatics.GetPlayerPawn` 0) false)
  (message `/Game/Definitions/Interfaces/BPI_DialogueControl.I_SetConversationLock` (`self.Target Actor`) false)
  (bind _widgetfield (message `/Game/Definitions/Interfaces/BPI_UIControl.I_GetWidgetField` (`GameplayStatics.GetPlayerController` 0)))
  (`/Game/UI/Widgets/WBP_Field.HideDialogue` _widgetfield))

(fn `ProcessDialogueLine`
  (params (RowName :type Name) (TargetActor :type "Actor Object Reference"))
  (returns (FoundRow :type Boolean))
  (bind (_message _nextrow _isplayer) (break `/Game/Definitions/Structs/DataTables/S_DialogueData` (`self.CurrentDialogueLine`)))
  (bind _returnvalue (`|GetDataTableRow` "/Game/Data/DataTables/DT_Dialogue.DT_Dialogue" (`local.RowName`))
    (:`then`
      (set `self.CurrentDialogueLine` _returnvalue)
      (set `self.Target Actor` (`local.TargetActor`))
      (bind _widgetfield (message `/Game/Definitions/Interfaces/BPI_UIControl.I_GetWidgetField` (`GameplayStatics.GetPlayerController` 0)))
      (`/Game/UI/Widgets/WBP_Field.ShowDialogue` _widgetfield (select `bool` _isplayer :`false` (`local.TargetActor`) :`true` (`GameplayStatics.GetPlayerPawn` 0) :!type "Actor Object Reference") _message)
      (return true))
    (:`RowNotFound`
      (return false))))

(fn `ProgressConversation`
  (bind ((`NextRow_5_EAECB49D488CE47CDEA3F68C4F634286` _nextrow)) (break `/Game/Definitions/Structs/DataTables/S_DialogueData` (`self.CurrentDialogueLine`)))
  (if (== (`.NextRow_5_EAECB49D488CE47CDEA3F68C4F634286` (break `/Game/Definitions/Structs/DataTables/S_DialogueData` (`self.CurrentDialogueLine`))) "None")
    (`self.EndConversation`)
    (else
      (bind _foundrow (`self.ProcessDialogueLine` _nextrow (`self.Target Actor`)))
      (if (not _foundrow)
        (`KismetSystemLibrary.PrintText` (`|FormatText` "Line Not Found: {Row}" _nextrow) true true (struct :`R` 1.0 :`G` 0.038421 :`A` 1.0) 5.0)
        (`self.EndConversation`)))))

(fn `StartConversation`
  (params (ConversationTarget :type "/Game/Blueprints/Field/NPCs/BP_NPC Object Reference") (RowName :type Name))
  (bind _foundrow (`self.ProcessDialogueLine` (`local.RowName`) (`local.ConversationTarget`)))
  (if _foundrow
    (message `/Game/Definitions/Interfaces/BPI_DialogueControl.I_SetConversationLock` (`GameplayStatics.GetPlayerPawn` 0) true)
    (message `/Game/Definitions/Interfaces/BPI_DialogueControl.I_SetConversationLock` (`local.ConversationTarget`) true)))