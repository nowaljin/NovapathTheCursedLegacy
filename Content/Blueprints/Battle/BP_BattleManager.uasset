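; Possessed pawn that runs a turn-based battle between spawned warriors and slimes, with a swaying camera.
; Turn order lists party then enemies and refills when empty, updating the turn-order UI.
; Party members slide forward via timelines and open the action menu, while enemy turns just wait and pass.
; Enhanced Input drives enemy target picking; accept only prints, and returning to the field level is currently unwired.
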(event `self.ReceiveBeginPlay`
  (message `/Game/Definitions/Interfaces/BPI_UIControl.I_InitWidgetBattle` (`GameplayStatics.GetPlayerController` 0))
  (`self.StartBattle`))

(event `self.ReceivePossessed`
  (params (NewController :type "Controller Object Reference"))
  (bind _asplayer_controller (cast `PlayerController` (`self.GetController`)))
  (`EnhancedInputSubsystemInterface.AddMappingContext` (pcsubsystem `EnhancedInputLocalPlayerSubsystem` _asplayer_controller) "/Game/Inputs/BattleNav/IMC_BattleNav.IMC_BattleNav" 0 (struct)))

(event `StartCameraSway`
  (bind (_relativerotation_roll _relativerotation_pitch) (`KismetMathLibrary.BreakRotator` (`SceneComponent.RelativeRotation` (`self.Camera`))))
  (`TimelineComponent.SetPlayRate` (`self.AnimCameraSway`) (`self.CameraSwayRate`))
  (bind (_direction _yawrotation) (`Timeline|AnimCameraSway` :!via `PlayFromStart`)
    (:`Update`
      (`SceneComponent.K2_SetRelativeRotation` (`self.Camera`) (`KismetMathLibrary.MakeRotator` _relativerotation_roll _relativerotation_pitch (* _yawrotation (`self.CameraSwayDistance`))) false false))))

(event `StartBattle`
  (for _array_element (`self.EnemyTeamLocations`)
    (bind _returnvalue (`|SpawnActorFromClass` "/Game/Blueprints/Battle/BattleChars/Enemies/Slime/BP_BattleSlime.BP_BattleSlime_C" (`KismetMathLibrary.MakeTransform` (+ _array_element (`self.SpawnHeightOffset`) (`self.K2_GetActorLocation`))) "AlwaysSpawn" "MultiplyWithRoot" null null))
    (`KismetArrayLibrary.Array_AddUnique` (`self.EnemyTeam`) _returnvalue))
  (for (_array_element_2 _array_index) (`self.PartyTeamLocations`)
    (bind _returnvalue_2 (`|SpawnActorFromClass` "/Game/Blueprints/Battle/BattleChars/Party/Warrior/BP_BattleWarrior.BP_BattleWarrior_C" (`KismetMathLibrary.MakeTransform` (+ _array_element_2 (`self.SpawnHeightOffset`) (`self.K2_GetActorLocation`)) (`self.PartyTeamRotation`)) "AlwaysSpawn" "MultiplyWithRoot" null null))
    (`KismetArrayLibrary.Array_AddUnique` (`self.PartyTeam`) _returnvalue_2)
    (bind _widgetbattle (message `/Game/Definitions/Interfaces/BPI_UIControl.I_GetWidgetBattle` (`GameplayStatics.GetPlayerController` 0)))
    (bind _aswbp_battle_health_mana (`/Game/UI/Widgets/Battle/WBP_PartyHealthManaPanel.GetCharWidget` (`/Game/UI/Widgets/WBP_Batle.WBP_PartyHealthManaPanel` _widgetbattle) _array_index))
    (`/Game/Blueprints/Battle/BattleChars/BP_BattleChar_BASE.AssignBattleHealthManaWidget` _returnvalue_2 _aswbp_battle_health_mana))
  (`self.DecideTurnOrder`)
  (`self.SelectActiveCharacter`)
  (`self.StartCameraSway`)
  (`Controller.Possess` (`GameplayStatics.GetPlayerController` 0) self)
  (`self.StartTurn`))

(event `ConcludeBattle`
  (bind _playerfieldposition (message `/Game/Definitions/Interfaces/BPI_InstanceStorage.I_GetPlayerFieldPosition` (`GameplayStatics.GetGameInstance`)))
  (`GameplayStatics.OpenLevel` (`KismetStringLibrary.Conv_StringToName` (`.FieldLevelName_2_5E5D1D9148ABB73C9689E39093EB6D36` (break `/Game/Definitions/Structs/S_FieldPosition` _playerfieldposition)))))

(event `StartTurn`
  (`KismetSystemLibrary.PrintString` (`KismetStringLibrary.Concat_StrStr` (`KismetSystemLibrary.GetDisplayName` (`self.ActiveCharacter`)) "is active!"))
  (if (`/Game/Blueprints/Battle/BattleChars/BP_BattleChar_BASE.IsPartyMember` (`self.ActiveCharacter`))
    (`self.MoveToActive`)
    (else
      (`KismetSystemLibrary.Delay` 2.0)
      (`self.ConcludeTurn`))))

(event `MoveToActive`
  ;[0.9646 0.9906 0 0.5] Move To Active
  (`/Game/UI/Widgets/Battle/WBP_BattleHealthMana.SlideOutAnim` (`/Game/Blueprints/Battle/BattleChars/BP_BattleChar_BASE.WidgetHealthMana` (`self.ActiveCharacter`)))
  (`TimelineComponent.SetPlayRate` (`self.AnimMoveToActive`) 2.0)
  (bind (_direction _alpha) (`Timeline|AnimMoveToActive` :!via `PlayFromStart`)
    (:`Update`
      (`self.K2_SetActorLocation` (`self.ActiveCharacter`) (`KismetMathLibrary.VLerp` (`/Game/Blueprints/Battle/BattleChars/BP_BattleChar_BASE.SpawnedLocation` (`self.ActiveCharacter`)) (`self.AdjustedActiveLocation`) _alpha) false false))
    (:`Finished`
      (bind _widgetbattle (message `/Game/Definitions/Interfaces/BPI_UIControl.I_GetWidgetBattle` (`GameplayStatics.GetPlayerController` 0)))
      (`/Game/UI/Widgets/Battle/WBP_ActionMenu.SetActionMenuVisible` (`/Game/UI/Widgets/WBP_Batle.WBP_ActionMenu` _widgetbattle) true self))))

(event `MoveBackFromActive`
  ;[0.9646 0.9906 0 0.5] Move Back From Active
  (`/Game/UI/Widgets/Battle/WBP_BattleHealthMana.SlideBackAnim` (`/Game/Blueprints/Battle/BattleChars/BP_BattleChar_BASE.WidgetHealthMana` (`self.ActiveCharacter`)))
  (bind _widgetbattle (message `/Game/Definitions/Interfaces/BPI_UIControl.I_GetWidgetBattle` (`GameplayStatics.GetPlayerController` 0)))
  (`/Game/UI/Widgets/Battle/WBP_ActionMenu.SetActionMenuVisible` (`/Game/UI/Widgets/WBP_Batle.WBP_ActionMenu` _widgetbattle) false null)
  (`TimelineComponent.SetPlayRate` (`self.AnimMoveBackFromActive`) 2.0)
  (bind (_direction _alpha) (`Timeline|AnimMoveBackFromActive` :!via `PlayFromStart`)
    (:`Update`
      (`self.K2_SetActorLocation` (`self.ActiveCharacter`) (`KismetMathLibrary.VLerp` (`self.AdjustedActiveLocation`) (`/Game/Blueprints/Battle/BattleChars/BP_BattleChar_BASE.SpawnedLocation` (`self.ActiveCharacter`)) _alpha) false false))
    (:`Finished`
      (`KismetSystemLibrary.Delay` 1.0)
      (`self.ConcludeTurn`))))

(event `ConcludeTurn`
  (`/Game/Blueprints/Battle/BattleChars/BP_BattleChar_BASE.HideBattlePortait` (`self.ActiveCharacter`))
  (`KismetArrayLibrary.Array_Remove` (`self.TurnOrder`))
  (if (`KismetArrayLibrary.Array_IsEmpty` (`self.TurnOrder`))
    (`self.DecideTurnOrder`)
    (`self.SelectActiveCharacter`)
    (`self.StartTurn`)
    (else
      (`self.SelectActiveCharacter`)
      (`self.StartTurn`))))

(event `EnhancedInput|/Game/Inputs/BattleNav/Actions/IA_BattleNav_Left`
  (params (ActionValue :type Boolean) (ElapsedSeconds :type "Float (double-precision)") (TriggeredSeconds :type "Float (double-precision)") (InputAction :type "InputAction Object Reference" :default "/Game/Inputs/BattleNav/Actions/IA_BattleNav_Left.IA_BattleNav_Left"))
  (:`Started`
    (if (`self.CanBattleNav`)
      (`self.MoveTargetPointer` false))))

(event `EnhancedInput|/Game/Inputs/BattleNav/Actions/IA_BattleNav_Right`
  (params (ActionValue :type Boolean) (ElapsedSeconds :type "Float (double-precision)") (TriggeredSeconds :type "Float (double-precision)") (InputAction :type "InputAction Object Reference" :default "/Game/Inputs/BattleNav/Actions/IA_BattleNav_Right.IA_BattleNav_Right"))
  (:`Started`
    (if (`self.CanBattleNav`)
      (`self.MoveTargetPointer` true))))

(event `EnhancedInput|/Game/Inputs/BattleNav/Actions/IA_BattleNav_Accept`
  (params (ActionValue :type Boolean) (ElapsedSeconds :type "Float (double-precision)") (TriggeredSeconds :type "Float (double-precision)") (InputAction :type "InputAction Object Reference" :default "/Game/Inputs/BattleNav/Actions/IA_BattleNav_Accept.IA_BattleNav_Accept"))
  (:`Started`
    (if (`self.CanBattleNav`)
      (`KismetSystemLibrary.PrintString` "Accept"))))

(event `EnhancedInput|/Game/Inputs/BattleNav/Actions/IA_BattleNav_Back`
  (params (ActionValue :type Boolean) (ElapsedSeconds :type "Float (double-precision)") (TriggeredSeconds :type "Float (double-precision)") (InputAction :type "InputAction Object Reference" :default "/Game/Inputs/BattleNav/Actions/IA_BattleNav_Back.IA_BattleNav_Back"))
  (:`Started`
    (if (`self.CanBattleNav`)
      (`self.EndTargetPickMode`))))

(fn `DecideTurnOrder`
  (`KismetArrayLibrary.Array_Clear` (`self.TurnOrder`))
  (`KismetArrayLibrary.Array_Append` (`self.TurnOrder`) (`self.PartyTeam`))
  (`KismetArrayLibrary.Array_Append` (`self.TurnOrder`) (`self.EnemyTeam`))
  ; Update UI
  (bind _widgetbattle (message `/Game/Definitions/Interfaces/BPI_UIControl.I_GetWidgetBattle` (`GameplayStatics.GetPlayerController` 0)))
  (`/Game/UI/Widgets/Battle/WBP_TurnOrder.ReplaceTurnOrder` (`/Game/UI/Widgets/WBP_Batle.WBP_TurnOrder` _widgetbattle) (`self.TurnOrder`)))

(fn `EndTargetPickMode`
  (`/Game/Blueprints/Battle/BattleChars/BP_BattleChar_BASE.SetPointerVisibility` (`self.Target`) false)
  (set `self.TargetIndex` 0)
  (set `self.CanBattleNav` false)
  (bind _widgetbattle (message `/Game/Definitions/Interfaces/BPI_UIControl.I_GetWidgetBattle` (`GameplayStatics.GetPlayerController` 0)))
  (`/Game/UI/Widgets/Battle/WBP_ActionMenu.SetActionMenuVisible` (`/Game/UI/Widgets/WBP_Batle.WBP_ActionMenu` _widgetbattle) true self))

(fn `MoveTargetPointer`
  (params (MoveRight :type Boolean))
  (`/Game/Blueprints/Battle/BattleChars/BP_BattleChar_BASE.SetPointerVisibility` (`self.Target`) false)
  (if (`local.MoveRight`)
    (`/Engine/EditorBlueprintResources/StandardMacros.IncrementInt` (`self.TargetIndex`)
      (:`  `
        _))
    (else
      (`/Engine/EditorBlueprintResources/StandardMacros.DecrementInt` (`self.TargetIndex`)
        (:`  `
          _))))
  (set `self.TargetIndex` (`KismetMathLibrary.Clamp` (`self.TargetIndex`) 0 (`KismetArrayLibrary.Array_LastIndex` (`self.EnemyTeam`))))
  (set `self.Target` (`|GetArrayItem` (`self.EnemyTeam`) (`self.TargetIndex`)))
  (`/Game/Blueprints/Battle/BattleChars/BP_BattleChar_BASE.SetPointerVisibility` (`self.Target`) true))

(fn `SelectActiveCharacter`
  (set `self.ActiveCharacter` (`|GetArrayItem` (`self.TurnOrder`))))

(fn `StartTargetPickMode`
  (set `self.Target` (`|GetArrayItem` (`self.EnemyTeam`)))
  (`/Game/Blueprints/Battle/BattleChars/BP_BattleChar_BASE.SetPointerVisibility` (`self.Target`) true)
  (bind _widgetbattle (message `/Game/Definitions/Interfaces/BPI_UIControl.I_GetWidgetBattle` (`GameplayStatics.GetPlayerController` 0)))
  (`/Game/UI/Widgets/Battle/WBP_ActionMenu.SetActionMenuVisible` (`/Game/UI/Widgets/WBP_Batle.WBP_ActionMenu` _widgetbattle) false null)
  (message `/Game/Definitions/Interfaces/BPI_UIControl.I_DeactivateUIControls` (`GameplayStatics.GetPlayerController` 0))
  (set `self.CanBattleNav` true))

(fn `UserConstructionScript`)