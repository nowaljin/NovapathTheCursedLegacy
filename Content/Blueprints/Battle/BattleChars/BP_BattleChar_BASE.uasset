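; Base actor for battle characters, handling attack presentation, hit reaction and the character's battle UI.
; Attacks play the data-defined override animation then, after a delay, have BattleManager move back from active; without one, a timeline hop plays and notifies the manager.
; Executing effects is delegated to BattleManager, while receiving one only shakes the sprite through ACShaker.
; It also toggles the target pointer, hides the portrait and activates the health/mana widget with placeholder current values.
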(event `self.ReceiveBeginPlay`
  (`|ExecutionSequence`
    (:`then_0`
      (set `self.SpawnedLocation` (`self.K2_GetActorLocation`))
      (bind _aswbp_target_pointer (cast `/Game/UI/Widgets/WBP_TargetPointer` (`WidgetComponent.GetUserWidgetObject` (`self.WidgetPointer`))))
      (set `self.WidgetTarget Pointer` _aswbp_target_pointer))
    (:`then_1`
      (`/Game/Blueprints/Components/AC_Shaker.Initialize` (`self.AC_Shaker`) (`self.Sprite`)))))

(event `PlayAttackAnim`
  (bind (_spawnedlocation_x _spawnedlocation_y _spawnedlocation_z) (`KismetMathLibrary.BreakVector` (`self.SpawnedLocation`)))
  (bind _attackanimdefault (`/Game/Data/DataAssets/BattleCharData/PDA_BattleCharData.AttackAnimDefault` (`self.BattleCharData`))
    (:`then`
      (`PaperZDPlaySlotOverrideAction.PlayAnimationOverrideWithCallbacks` (`PaperZDAnimationComponent.AnimInstance` (`self.AnimationComponent`)) _attackanimdefault
        (:`OnCompleted`
          _)
        (:`OnCancelled`
          _))
      (`KismetSystemLibrary.RetriggerableDelay` (`self.AfterAttackDelay`))
      (`/Game/Blueprints/Battle/BP_BattleManager.MoveBackFromActive` (`self.BattleManager`)))
    (:`else`
      (`TimelineComponent.SetPlayRate` (`self.AnimDoubleJump`) (`self.JumpPlayRate`))
      (bind (_direction _alpha) (`Timeline|AnimDoubleJump` :!via `PlayFromStart`)
        (:`Update`
          (`self.K2_SetActorLocation` (`KismetMathLibrary.MakeVector` _spawnedlocation_x _spawnedlocation_y (+ _spawnedlocation_z (* _alpha (`self.JumpHeight`))))))
        (:`Finished`
          (`/Game/Blueprints/Battle/BP_BattleManager.FinishedTimeLineAttackAnim` (`self.BattleManager`)))))))

(fn `AssignBattleHealthManaWidget`
  (params (WidgetHealthMana :type "/Game/UI/Widgets/Battle/WBP_BattleHealthMana Object Reference"))
  (bind _battlechardata (`self.BattleCharData`))
  (bind (_maxhp _maxmp) (break `/Game/Definitions/Structs/S_CharAttributes` (`/Game/Data/DataAssets/BattleCharData/PDA_BattleCharData.InitialAttributes` _battlechardata)))
  (set `self.WidgetHealthMana` WidgetHealthMana)
  (`/Game/UI/Widgets/Battle/WBP_BattleHealthMana.Activate` (`self.WidgetHealthMana`) (`/Game/Data/DataAssets/BattleCharData/PDA_BattleCharData.DisplayName` _battlechardata) _maxhp 10.0 _maxmp 10.0))

(fn `ExecuteBattleEffect`
  (`/Game/Blueprints/Battle/BP_BattleManager.ApplyBattleEffect` (`self.BattleManager`)))

(fn `HideBattlePortait`
  (bind _widgetportrait (`self.WidgetPortrait`)
    (:`then`
      (`/Game/UI/Widgets/Battle/WBP_Portrait.HidePortrait` _widgetportrait)
      (set `self.WidgetPortrait` null))
    (:`else`)))

(fn `ReceiveBattleEffect`
  (`/Game/Blueprints/Components/AC_Shaker.StartShake` (`self.AC_Shaker`)))

(fn `SetPointerVisibility`
  (params (SetVisible :type Boolean))
  (if SetVisible
    (`/Game/UI/Widgets/WBP_TargetPointer.ShowPointer` (`self.WidgetTarget Pointer`))
    (else
      (`/Game/UI/Widgets/WBP_TargetPointer.HidePointer` (`self.WidgetTarget Pointer`)))))

(fn `UserConstructionScript`)