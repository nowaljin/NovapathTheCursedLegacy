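; GI_Core is the game instance blueprint that holds shared state: global variables, party members and the player's field position.
; An interface event records the last field transform, then adds the current level name and area data queried from the game mode through an interface.
; Interface getters expose all three pieces of state to other objects.
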(event `/Game/Definitions/Interfaces/BPI_InstanceStorage.I_StoreFieldPosition`
  (params (LastFieldTransform :type "Transform Structure"))
  (`self.StoreFieldPosition` LastFieldTransform))

(fn `I_GetGlobalVariables`
  (returns (GlobalVariables :type "/Game/Data/DataAssets/GlobalVariables/PDA_GlobalVariables Object Reference"))
  (return (`self.GlobalVariables`)))

(fn `I_GetPartyMembers`
  (returns (PartyMembers :type "Array of /Game/Data/DataAssets/PartyMemberData/PDA_PartyMemberData Object Reference"))
  (return (`self.PartyMembers`)))

(fn `I_GetPlayerFieldPosition`
  (returns (PlayerFieldPosition :type "/Game/Definitions/Structs/S_FieldPosition Structure"))
  (return (`self.PlayerFieldPosition`)))

(fn `StoreFieldPosition`
  (params (LastFieldTransform :type "Transform Structure"))
  (setmembers `/Game/Definitions/Structs/S_FieldPosition` :`StructRef` (`self.PlayerFieldPosition`) :`LastFieldTransform` LastFieldTransform)
  (bind _areadata (message `/Game/Definitions/Interfaces/BPI_AreaControl.I_GetCurrentAreaData` (`GameplayStatics.GetGameMode`)))
  (bind _returnvalue (`GameplayStatics.GetCurrentLevelName` true))
  (setmembers `/Game/Definitions/Structs/S_FieldPosition` :`StructRef` (`self.PlayerFieldPosition`) :`FieldLevelName` _returnvalue :`AreaInfo` _areadata))